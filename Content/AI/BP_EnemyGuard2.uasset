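; Enemy guard character that can be armed, feeds its AI Blackboard from perception and fires bullets from its muzzle.
; Hearing writes a noise location; sight sets target, visibility and last seen position and raises walk speed, which drops when the target is forgotten.
; On BeginPlay, the Armed flag sets rifle visibility and aim pose.
; Health changes update a widget bar, and death disables capsule collision and movement and ragdolls the mesh.
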(event OnTargetPerceptionForgotten(AIPerception)
  (params (Actor :type Actor%20Object%20Reference))
  (Variables|/Script/Engine.CharacterMovementComponent|SetMaxWalkSpeed (Variables|Character|GetCharacterMovement) 2e+02)
  (AI|Components|Blackboard|ClearValue (AI|GetBlackboard (AI|GetAIController self)) (Utilities|Name|MakeLiteralName "TargetActor")))

(event OnTargetPerceptionUpdated(AIPerception)
  (params (Actor :type Actor%20Object%20Reference) (Stimulus :type AI%20Stimulus%20Structure))
  (bind (_age _expirationage _strength _stimuluslocation _receiverlocation _tag _bsuccessfullysensed) (Utilities|Struct|BreakAIStimulus Stimulus))
  (bind _self self)
  (bind _returnvalue (AI|GetAIController _self))
  (bind _returnvalue_2 (AI|GetBlackboard _returnvalue))
  (bind _returnvalue_3 (Class|AIPerceptionSystem|GetSenseClassforStimulus Stimulus))
  (if (== _returnvalue_3 "/Script/AIModule.AISense_Hearing")
    (AI|Components|Blackboard|SetValueasVector (AI|GetBlackboard (AI|GetAIController self)) (Utilities|Name|MakeLiteralName "NoiseLocation") _stimuluslocation)
    (elif (== _returnvalue_3 "/Script/AIModule.AISense_Sight")
      (if _bsuccessfullysensed
        (AI|Components|Blackboard|SetValueasObject _returnvalue_2 (Utilities|Name|MakeLiteralName "TargetActor") Actor)
        (AI|Components|Blackboard|SetValueasBool _returnvalue_2 (Utilities|Name|MakeLiteralName "IsPlayerInSight") true)
        (AI|Components|Blackboard|SetValueasVector _returnvalue_2 (Utilities|Name|MakeLiteralName "LastSeenLocation") _stimuluslocation)
        (Variables|/Script/Engine.CharacterMovementComponent|SetMaxWalkSpeed (Variables|Character|GetCharacterMovement) 6e+02)
        (else
          (AI|Components|Blackboard|ClearValue _returnvalue_2 (Utilities|Name|MakeLiteralName "IsPlayerInSight")))))))

(event Custom|OnHealthChanged_Event
  (bind _mesh (Variables|Character|GetMesh))
  (bind _bp_healthcomponent (Variables|Default|GetBP_HealthComponent))
  (bind _ashealth_indicator (Utilities|Casting|CastToHealthIndicator (UserInterface|GetWidget (Variables|Default|GetWidget))))
  (Progress|SetPercent (Variables|/Game/UI/HealthIndicator.HealthIndicator_C|GetHealthProgressBar _ashealth_indicator) (Variables|/Game/Blueprins/BP_HealthComponent.BP_HealthComponent_C|GetHealthPercentage _bp_healthcomponent))
  (if (Variables|/Game/Blueprins/BP_HealthComponent.BP_HealthComponent_C|GetDied _bp_healthcomponent)
    (Collision|SetCollisionEnabled (Variables|Collision|GetCapsuleComponent) "NoCollision")
    (Collision|SetCollisionProfileName _mesh "Ragdoll" true :!class /Script/Engine.PrimitiveComponent)
    (Physics|SetSimulatePhysics _mesh true)
    (Pawn|Components|CharacterMovement|DisableMovement (Variables|Character|GetCharacterMovement))))

(event EventBeginPlay
  (CallFunction|ArmEnemy)
  (EventDispatchers|AssignOnHealthChanged (Variables|Default|GetBP_HealthComponent) (delegate Custom|OnHealthChanged_Event)))

(event EventFireEvent
  (Game|SpawnActorfromClass "/Game/AI/BP_Bullet.BP_Bullet_C" (Math|Transform|MakeTransform (Transformation|GetWorldLocation (Variables|Default|GetMuzzleArrow1)) (Transformation|GetWorldRotation (Variables|Collision|GetCapsuleComponent))) "Undefined" "MultiplyWithRoot" 0 0))

(fn ConstructionScript)

(fn ArmEnemy
  (bind _mesh (Variables|Character|GetMesh))
  (bind _rifle (Variables|Default|GetRifle))
  (bind _returnvalue (Components|SkeletalMesh|GetAnimInstance _mesh))
  (if (Variables|Default|GetArmed)
    (bind _asabp_unarmed (Utilities|Casting|CastToABP_Unarmed _returnvalue))
    (Variables|/Game/Characters/Mannequins/Anims/Unarmed/ABP_Unarmed.ABP_Unarmed_C|SetIsAiming _asabp_unarmed true)
    (Rendering|SetVisibility _rifle true false)
    (AI|Components|Blackboard|SetValueasBool (AI|GetBlackboard (AI|GetAIController self)) (Utilities|Name|MakeLiteralName "Armed") true)
    (else
      (bind _asabp_unarmed_2 (Utilities|Casting|CastToABP_Unarmed _returnvalue))
      (Variables|/Game/Characters/Mannequins/Anims/Unarmed/ABP_Unarmed.ABP_Unarmed_C|SetIsAiming _asabp_unarmed_2 false)
      (Rendering|SetVisibility _rifle false false))))