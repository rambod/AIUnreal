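; Enemy guard character that patrols between random tagged actors, pausing after each successful move, and reacts to AI perception.
; A "ball" stimulus sends it to the stimulus location, while other stimuli from the player character start a faster chase.
; Forgetting a target lowers its speed and resumes patrol.
; Health changes update its widget bar, and death disables capsule collision and movement and ragdolls the mesh.
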(event OnTargetPerceptionUpdated(AIPerception)
  (params (Actor :type Actor%20Object%20Reference) (Stimulus :type AI%20Stimulus%20Structure))
  (bind (_age _expirationage _strength _stimuluslocation _receiverlocation _tag) (Utilities|Struct|BreakAIStimulus Stimulus))
  (if (not (== _tag "ball"))
    (bind _asbp_third_person_character (Utilities|Casting|CastToBP_ThirdPersonCharacter Actor))
    (Variables|/Script/Engine.CharacterMovementComponent|SetMaxWalkSpeed (Variables|Character|GetCharacterMovement) 5e+02)
    (AI|AIMoveTo self "0, 0, 0" _asbp_third_person_character 5.0 false)
    (else
      (AI|AIMoveTo self _stimuluslocation 0 5.0 false))))

(event OnTargetPerceptionForgotten(AIPerception)
  (params (Actor :type Actor%20Object%20Reference))
  (Variables|/Script/Engine.CharacterMovementComponent|SetMaxWalkSpeed (Variables|Character|GetCharacterMovement) 3e+02)
  (bind _outactors (Actor|GetAllActorswithTag (Variables|Default|GetTag) :!label _label))
  (AI|AIMoveTo self "0, 0, 0" (.OutItem (Utilities|Array|Random _outactors)) 5.0 false
    (:OnSuccess
      (Utilities|FlowControl|Delay 2.0)
      (goto _label))))

(event Custom|OnTargetPerceptionForgotten_Event
  (params (Actor :type Actor%20Object%20Reference))
  (Development|PrintString (Utilities|String|ToString(Text) (Utilities|Text|FormatText "AI Forget this {actor}" Actor)))
  (Variables|/Script/Engine.CharacterMovementComponent|SetMaxWalkSpeed (Variables|Character|GetCharacterMovement) 3e+02)
  (bind _outactors (Actor|GetAllActorswithTag (Variables|Default|GetTag) :!label _label))
  (AI|AIMoveTo self "0, 0, 0" (.OutItem (Utilities|Array|Random _outactors)) 5.0 false
    (:OnSuccess
      (Utilities|FlowControl|Delay 2.0)
      (goto _label))))

(event Custom|OnHealthChanged_Event
  (bind _mesh (Variables|Character|GetMesh))
  (bind _bp_healthcomponent (Variables|Default|GetBP_HealthComponent))
  (bind _ashealth_indicator (Utilities|Casting|CastToHealthIndicator (UserInterface|GetWidget (Variables|Default|GetWidget))))
  (Progress|SetPercent (Variables|/Game/UI/HealthIndicator.HealthIndicator_C|GetHealthProgressBar _ashealth_indicator) (Variables|/Game/Blueprins/BP_HealthComponent.BP_HealthComponent_C|GetHealthPercentage _bp_healthcomponent))
  (if (Variables|/Game/Blueprins/BP_HealthComponent.BP_HealthComponent_C|GetDied _bp_healthcomponent)
    (Collision|SetCollisionEnabled (Variables|Collision|GetCapsuleComponent) "NoCollision")
    (Collision|SetCollisionProfileName _mesh "Ragdoll" true :!class /Script/Engine.PrimitiveComponent)
    (Physics|SetSimulatePhysics _mesh true)
    (Pawn|Components|CharacterMovement|DisableMovement (Variables|Character|GetCharacterMovement))))

(event EventBeginPlay
  (Utilities|FlowControl|Sequence
    (:then_0
      (EventDispatchers|AssignOnTargetPerceptionForgotten (Variables|Default|GetAIPerception) (delegate Custom|OnTargetPerceptionForgotten_Event))
      (bind _outactors (Actor|GetAllActorswithTag (Variables|Default|GetTag) :!label _label))
      (AI|AIMoveTo self "0, 0, 0" (.OutItem (Utilities|Array|Random _outactors)) 5.0 false
        (:OnSuccess
          (Utilities|FlowControl|Delay 2.0)
          (goto _label))))
    (:then_1
      (EventDispatchers|AssignOnHealthChanged (Variables|Default|GetBP_HealthComponent) (delegate Custom|OnHealthChanged_Event)))))

(fn ConstructionScript)